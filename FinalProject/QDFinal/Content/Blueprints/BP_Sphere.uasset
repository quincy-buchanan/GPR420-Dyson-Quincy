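; BP_Sphere is a collectible actor that adds to the player's collected sphere count.
; On BeginPlay it casts the first player character to BP_PlayerCharacter and caches the reference.
; Its Hit event increments SpheresCollected on that cached player without checking what hit it, then destroys the sphere.
; A debug print follows, showing one more than the stored count because it adds again after the increment.
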(event `self.ReceiveHit`
  (params (MyComp :type "PrimitiveComponent Object Reference") (Other :type "Actor Object Reference") (OtherComp :type "PrimitiveComponent Object Reference") (bSelfMoved :type Boolean) (HitLocation :type "Vector Structure") (HitNormal :type "Vector Structure") (NormalImpulse :type "Vector Structure") (Hit :type "HitResult Structure (by ref)"))
  (bind _player (`self.Player`))
  (bind _returnvalue (+ (`/Game/Blueprints/BP_PlayerCharacter.SpheresCollected` _player) 1))
  (set `/Game/Blueprints/BP_PlayerCharacter.SpheresCollected` _returnvalue _player)
  (`self.K2_DestroyActor`)
  (`KismetSystemLibrary.PrintString` (`KismetStringLibrary.Conv_IntToString` _returnvalue)))

(event `self.ReceiveBeginPlay`
  (bind _asbp_player_character (cast `/Game/Blueprints/BP_PlayerCharacter` (`GameplayStatics.GetPlayerCharacter` 0)))
  (set `self.Player` _asbp_player_character))

(fn `UserConstructionScript`)