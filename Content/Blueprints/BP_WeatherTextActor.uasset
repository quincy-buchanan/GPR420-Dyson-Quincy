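; Actor that displays the current short weather forecast for a fixed location in a text render component.
; On BeginPlay it uses the VaRest plugin to GET a hardcoded api.weather.gov gridpoint forecast.
; The callback parses the JSON and writes the first period's shortForecast to the text.
; Unconnected nodes hold an unused points lookup that would resolve the forecast URL from coordinates.
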(event `self.ReceiveBeginPlay`
  (bind _returnvalue (subsystem `VaRestSubsystem`))
  (bind _returnvalue_2 (`VaRestSubsystem.ConstructVaRestJsonObject` _returnvalue))
  (`VaRestSubsystem.CallURL` _returnvalue "https://api.weather.gov/gridpoints/BTV/88,56/forecast" "GET" "json" _returnvalue_2 (delegate `RestCallback`)))

(event `RestCallback`
  (params (Request :type "VaRestRequestJSON Object Reference"))
  (bind _returnvalue (`VaRestJsonValue.AsObject` (`VaRestJsonObject.GetField` (`VaRestRequestJSON.GetResponseObject` Request) "properties")))
  (bind _returnvalue_2 (`VaRestJsonValue.AsObject` (`|GetArrayItem` (`VaRestJsonObject.GetArrayField` _returnvalue "periods"))))
  (`TextRenderComponent.K2_SetText` (`self.TextRender`) (`KismetTextLibrary.Conv_StringToText` (`VaRestJsonObject.GetStringField` _returnvalue_2 "shortForecast"))))

(fn `UserConstructionScript`)