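; Light source Blueprint that tints its directional light according to a real-world temperature forecast from the US National Weather Service.
; On BeginPlay it sends a single VaRest GET request to api.weather.gov for a fixed BTV gridpoint.
; The callback reads the first forecast period's temperature and maps it linearly and inversely to light color temperature, so hotter forecasts give warmer light.
; An unconnected SetLightColor call never runs.
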(event `self.ReceiveBeginPlay`
  (bind _returnvalue (subsystem `VaRestSubsystem`))
  (bind _returnvalue_2 (`VaRestSubsystem.ConstructVaRestJsonObject` _returnvalue))
  (`VaRestSubsystem.CallURL` _returnvalue "https://api.weather.gov/gridpoints/BTV/88,56/forecast" "GET" "json" _returnvalue_2 (delegate `RestCallback`)))

(event `RestCallback`
  (params (Request :type "VaRestRequestJSON Object Reference"))
  (bind _returnvalue (`VaRestJsonValue.AsObject` (`VaRestJsonObject.GetField` (`VaRestRequestJSON.GetResponseObject` Request) "properties")))
  (bind _returnvalue_2 (`VaRestJsonValue.AsObject` (`|GetArrayItem` (`VaRestJsonObject.GetArrayField` _returnvalue "periods"))))
  (`LightComponent.SetTemperature` (`self.GetComponentByClass` "/Script/Engine.DirectionalLightComponent") (+ (* (- 100.0 (`KismetMathLibrary.Conv_IntToDouble` (`VaRestJsonObject.GetIntegerField` _returnvalue_2 "temperature"))) 103.0) 1700.0)))

(fn `UserConstructionScript`)